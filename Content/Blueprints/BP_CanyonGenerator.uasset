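; Procedural canyon generator actor that lays out two rows of scaled static mesh walls along a randomly jittered spline.
; The construction script rebuilds the spline with evenly spaced X points and random Y offsets, then adds left and right walls at each point, offset by the canyon width.
; Walls stay unrotated and use local spline positions as world transforms, so placement ignores the actor's transform.
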(event EventBeginPlay)

(event Collision|EventActorBeginOverlap
  (params (OtherActor :type Actor%20Object%20Reference)))

(event EventTick
  (params (DeltaSeconds :type Float%20%28single-precision%29)))

(fn ConstructionScript
  (Spline|ClearSplinePoints (Variables|Default|GetSpline) true)
  (|GenerateSplinePoints
    (:Completed
      (|GenerateLeftWalls
        (:Completed
          (|GenerateRightWalls))))))