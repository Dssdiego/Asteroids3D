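; BP_PlayerController moves a player-controlled mesh through thrust and tilt input axes, despite its name behaving like a pawn.
; Thrust and Tilt add movement along fixed world forward and right vectors, derived from a zero rotation rather than the actor's facing.
; Tilt also rotates the static mesh in local pitch, scaled by TiltSpeed.
; Mouse camera events are empty, and the spring-arm rotation and angle-clamping logic is disconnected.
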(event EventBeginPlay)

(event Collision|EventActorBeginOverlap
  (params (OtherActor :type Actor%20Object%20Reference)))

(event EventTick
  (params (DeltaSeconds :type Float%20%28single-precision%29)))

(event Input|AxisEvents|InputAxisThrust
  (params (AxisValue :type Float%20%28single-precision%29))
  ;[1 1 1] Thrusting
  (Pawn|Input|AddMovementInput (Math|Vector|GetForwardVector "0, 0, 0") AxisValue false))

(event Input|AxisEvents|InputAxisTilt
  (params (AxisValue :type Float%20%28single-precision%29))
  ;[1 1 1] Tilting (Left/Right)
  (Pawn|Input|AddMovementInput (Math|Vector|GetRightVector "0, 0, 0") AxisValue false)
  (Transformation|AddLocalRotation (Variables|Default|GetStaticMesh) (* (Math|Rotator|MakeRotator 0.0 (Input|AxisValues|GetTilt) 0.0) (Variables|Movement|GetTiltSpeed)) false false))

(event Input|MouseEvents|MouseX
  (params (AxisValue :type Float%20%28single-precision%29))
  ;[1 1 1] Camera X
)

(event Input|MouseEvents|MouseY
  (params (AxisValue :type Float%20%28single-precision%29))
  ;[1 1 1] Camera Y
)

(fn ConstructionScript)