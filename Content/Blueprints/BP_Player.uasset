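; BP_Player is the player ship, handling thrust, pitch and camera control through input axis and action events.
; Thrust offsets the actor along its forward vector by ThrustSpeed without sweep, and Pitch adds world-space rotation, neither scaled by delta time.
; The horizontal camera axis yaws the SpringArm locally, while the look-back action applies a half-turn with a pitch offset on both press and release.
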(event Input|ActionEvents|InputActionCameraLookBack
  (params (Key :type Key%20Structure :default "None"))
  ;[1 1 1] [Camera] Look Back
  (:Pressed
    (Transformation|AddLocalRotation (Variables|Default|GetSpringArm) "-30.000000,180.000000, 0" false false))
  (:Released
    (Transformation|AddLocalRotation (Variables|Default|GetSpringArm) "-30.000000,-180.000000, 0" false false)))

(event Input|AxisEvents|InputAxisThrust
  (params (AxisValue :type Float%20%28single-precision%29))
  ;[1 1 1] [Ship] Thrusting
  (Transformation|AddActorWorldOffset (* (Transformation|GetActorForwardVector) (* AxisValue (Variables|Movement|GetThrustSpeed)))))

(event Input|AxisEvents|InputAxisPitch
  (params (AxisValue :type Float%20%28single-precision%29))
  ;[1 1 1] [Ship] Pitch Rotation
  (Class|Actor|AddActorWorldRotation (Math|Rotator|MakeRotator 0.0 AxisValue 0.0)))

(event Input|AxisEvents|InputAxisCameraHorizontal
  (params (AxisValue :type Float%20%28single-precision%29))
  ;[1 1 1] [Camera] Horizontal Rotation (Yaw)
  (Transformation|AddLocalRotation (Variables|Default|GetSpringArm) (Math|Rotator|MakeRotator 0.0 0.0 AxisValue) false false))

(fn ConstructionScript)