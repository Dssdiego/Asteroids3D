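; BP_Player_Physics is a player-controlled ship that rotates through physics.
; Roll, pitch and yaw inputs apply torque about the root's local axes, scaled by ShipMoveSpeed.
; Tick damps spin with counter-torque from angular velocity divided by ShipMoveFrictionProportion.
; Thrust bypasses physics with an unswept, delta-time-scaled offset along actor forward, while spring-arm camera rotation nodes are left disconnected.
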(event EventTick
  (params (DeltaSeconds :type Float%20%28single-precision%29))
  ;[1 1 1] [Ship] Movement Friction
  (Class|PrimitiveComponent|AddTorqueinDegrees (Variables|Default|GetRoot) (/ (Math|Vector|NegateVector (Physics|GetPhysicsAngularVelocityinDegrees (Variables|Default|GetRoot) "None")) (Variables|Movement|GetShipMoveFrictionProportion)) "None" true))

(event Input|ActionEvents|InputActionCameraLookBack
  (params (Key :type Key%20Structure :default "None"))
  ;[1 1 1] [Camera] Look Back
)

(event Input|AxisEvents|InputAxisThrust
  (params (AxisValue :type Float%20%28single-precision%29))
  ;[1 1 1] [Ship] Thrusting
  (Transformation|AddActorWorldOffset (* (* (Transformation|GetActorForwardVector) (* AxisValue (Variables|Movement|GetShipMoveSpeed))) (Utilities|Time|GetWorldDeltaSeconds))))

(event Input|AxisEvents|InputAxisCameraHorizontal
  (params (AxisValue :type Float%20%28single-precision%29))
  ;[1 1 1] [Camera] Horizontal Rotation (Yaw)
)

(event Input|AxisEvents|InputAxisRoll
  (params (AxisValue :type Float%20%28single-precision%29))
  ;[1 1 1] [Ship] Roll
  (Class|PrimitiveComponent|AddTorqueinDegrees (Variables|Default|GetRoot) (* (Math|Vector|GetForwardVector (Variables|Default|GetRoot)) (* AxisValue (Variables|Movement|GetShipMoveSpeed))) "None" true))

(event Input|AxisEvents|InputAxisYaw
  (params (AxisValue :type Float%20%28single-precision%29))
  ;[1 1 1] [Ship] Yaw
  (Class|PrimitiveComponent|AddTorqueinDegrees (Variables|Default|GetRoot) (* (Math|Vector|GetUpVector (Variables|Default|GetRoot)) (* AxisValue (Variables|Movement|GetShipMoveSpeed))) "None" true))

(event Input|AxisEvents|InputAxisPitch
  (params (AxisValue :type Float%20%28single-precision%29))
  ;[1 1 1] [Ship] Pitch
  (Class|PrimitiveComponent|AddTorqueinDegrees (Variables|Default|GetRoot) (* (Math|Vector|GetRightVector (Variables|Default|GetRoot)) (* AxisValue (Variables|Movement|GetShipMoveSpeed))) "None" true))

(fn ConstructionScript)